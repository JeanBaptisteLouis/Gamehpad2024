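; BP_TheTribute is a one-shot interactable level element built around the CornichonMoisis component.
; While it is interactable, being looked at turns on the component's custom depth rendering as a highlight.
; Interacting passes TheTribute to Launch on the first-person character's AsBPSceneIncrducul reference, then disables further interaction and destroys the NStars component.
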(event `self.LookAt`
  (params (look :type Boolean))
  (`PrimitiveComponent.SetRenderCustomDepth` (`self.cornichon_moisis`) (and (`self.Interactable`) look)))

(event `self._Interact`
  (bind _asbp_first_person_character (cast `/Game/FirstPerson/Blueprints/BP_FirstPersonCharacter` (`GameplayStatics.GetPlayerCharacter` 0)))
  (`/Game/FirstPerson/Blueprints/BP_SceneIncrducul.Launch` (`/Game/FirstPerson/Blueprints/BP_FirstPersonCharacter.As BP Scene Incrducul` _asbp_first_person_character) "/Game/Collectibles/TheTribute.TheTribute")
  (set `self.Interactable` false)
  (`ActorComponent.K2_DestroyComponent` (`self.N_Stars`)))

(fn `UserConstructionScript`
  (`parent.UserConstructionScript`))