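; BP_Interactable is an interactable cube level element that highlights when looked at and spins when used.
; Lookat toggles the cube's custom depth rendering, likely for an outline effect.
; The _Interact event flip-flops a timeline between play and reverse, sweeping the cube through a full pitch rotation and back.
; The Interact function triggers the interaction and returns true.
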(event `/Game/Global/Blueprint/BPI_Interact.LookAt`
  (params (look :type Boolean))
  (`PrimitiveComponent.SetRenderCustomDepth` (`self.Cube`) look))

(event `_Interact`
  (`/Engine/EditorBlueprintResources/StandardMacros.FlipFlop`
    (:`A`
      (bind (_direction _alpha) (`Timeline|Timeline` :!label _label)
        (:`Update`
          (`SceneComponent.K2_SetRelativeRotation` (`self.Cube`) (`KismetMathLibrary.MakeRotator` 0.0 (* _alpha 360.0)) false false))))
    (:`B`
      (goto _label :!via `Reverse`))))

(fn `Interact`
  (returns (interacted :type Boolean))
  (`self._Interact`)
  (return true))

(fn `UserConstructionScript`)