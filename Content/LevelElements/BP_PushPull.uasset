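; BP_PushPull is an interactable cube that the player pushes back and forth between its origin and a Target offset.
; On Interact, a dot product checks that the player stands on the pushing side, which swaps with the Moved state.
; A valid push flips a FlipFlop that plays or reverses a timeline lerping the cube's location.
; Otherwise, a second timeline tilts the cube around an axis perpendicular to the player's direction as feedback.
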(event `self._Interact`
  (bind _returnvalue (`self.K2_GetActorLocation`))
  (bind _returnvalue_2 (`KismetMathLibrary.TransformLocation` (`self.GetTransform`) (`self.Target`)))
  (if (> (`KismetMathLibrary.Dot_VectorVector` (`KismetMathLibrary.Normal` (- (`self.K2_GetActorLocation` (`GameplayStatics.GetPlayerCharacter` 0)) (`SceneComponent.K2_GetComponentLocation` (`self.Cube`)))) (`KismetMathLibrary.SelectVector` (`KismetMathLibrary.Normal` (- _returnvalue_2 _returnvalue)) (`KismetMathLibrary.Normal` (- _returnvalue _returnvalue_2)) (`self.moved`))) 0.5)
    (`/Engine/EditorBlueprintResources/StandardMacros.FlipFlop`
      (:`A`
        (set `self.moved` true)
        (bind (_direction _alpha) (`Timeline|Timeline_2` :!label _label)
          (:`Update`
            (`SceneComponent.K2_SetRelativeLocation` (`self.Cube`) (`KismetMathLibrary.VLerp` (0.0 0.0 0.0) (`self.Target`) _alpha) false false))))
      (:`B`
        (set `self.moved` false)
        (goto _label :!via `Reverse`)))
    (else
      (bind _output_get (set `self.NewVar` (`KismetMathLibrary.GreaterGreater_VectorRotator` (`KismetMathLibrary.Normal` (- (`self.K2_GetActorLocation` (`GameplayStatics.GetPlayerCharacter` 0)) (`SceneComponent.K2_GetComponentLocation` (`self.Cube`)))) (struct :`Yaw` -90.0))))
      (bind (_direction_2 _alpha_2) (`Timeline|Timeline_0` :!via `PlayFromStart`)
        (:`Update`
          (`SceneComponent.K2_SetRelativeRotation` (`self.Cube`) (* (`KismetMathLibrary.RotatorFromAxisAndAngle` _output_get 5.0) _alpha_2) false false))))))

(fn `UserConstructionScript`
  (`parent.UserConstructionScript`))