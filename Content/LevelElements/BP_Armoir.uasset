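; BP_Armoir is an armoire level element that slides to a new position when its Interact event fires.
; Interact converts the local NewPosition offset to world space, saves it, and plays the LinearTranslation timeline from the start.
; Each update lerps from the current location rather than a stored start, without sweep, so movement compounds toward the target.
; Each interaction recomputes the target from the current transform, with no reverse path.
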(event `self._Interact`
  ;[0 1 0.9536] Linear Translation Movement
  (set `self.NewPositionSave` (`KismetMathLibrary.TransformLocation` (`self.GetTransform` self) (`self.NewPosition`)))
  (bind (_direction _newtrack_1) (`Timeline|LinearTranslation` :!via `PlayFromStart`)
    (:`Update`
      (`self.K2_SetActorLocation` (`KismetMathLibrary.VLerp` (`self.K2_GetActorLocation`) (`self.NewPositionSave`) _newtrack_1)))))

(fn `UserConstructionScript`
  (`parent.UserConstructionScript`))