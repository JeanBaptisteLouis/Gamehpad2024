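; Interactable can that, on Interact, travels in a straight line to a destination set in its local space while its mesh rolls.
; A timeline lerps both actor location, without sweep, and mesh pitch.
; Roll angle comes from travel distance over the mesh bounds' circumference, with direction set by the destination's X sign.
; The construction script strips actor pitch and roll, keeping only yaw.
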(event `self._Interact`
  (bind (_oldrotation_roll _oldrotation_pitch) (`KismetMathLibrary.BreakRotator` (`self.OldRotation`)))
  (bind (_oldrotation_roll_2 _oldrotation_pitch_2 _oldrotation_yaw) (`KismetMathLibrary.BreakRotator` (`self.OldRotation`)))
  (bind _returnvalue (+ _oldrotation_pitch (* 360.0 (/ (`KismetMathLibrary.Vector_Distance` (`self._ActorPositionSave`) (`self._TargetDestinationSave`)) (* (* (.x (`.Max` (`StaticMeshComponent.GetLocalBounds` (`self.Cube`)))) 2.0) (`KismetMathLibrary.GetPI`))))))
  ;[0 1 0.9536] Linear Translation Movement + Mesh Anim
  (`self.F_SaveMovementDatas`)
  (bind (_direction _newtrack_1) (`Timeline|Timeline_0` :!via `PlayFromStart`)
    (:`Update`
      (`self.K2_SetActorLocation` (`KismetMathLibrary.VLerp` (`self._ActorPositionSave`) (`self._TargetDestinationSave`) _newtrack_1))
      (if (`self.Clockwise`)
        (set `self.RotationValue` _returnvalue)
        (else
          (set `self.RotationValue` (* _returnvalue -1.0))))
      (`SceneComponent.K2_SetRelativeRotation` (`self.Cube`) (`KismetMathLibrary.RLerp` (`self.OldRotation`) (`KismetMathLibrary.MakeRotator` _oldrotation_roll_2 (`self.RotationValue`) _oldrotation_yaw) _newtrack_1) false false))))

(fn `F_SaveMovementDatas`
  (bind _targetdestination_x (`KismetMathLibrary.BreakVector` (`self.TargetDestination`)))
  (set `self._ActorPositionSave` (`self.K2_GetActorLocation`))
  (set `self._TargetDestinationSave` (`KismetMathLibrary.TransformLocation` (`self.GetTransform` self) (`self.TargetDestination`)))
  (set `self.OldRotation` (`SceneComponent.RelativeRotation` (`self.Cube`)))
  (if (> _targetdestination_x 0.0)
    (set `self.Clockwise` false)
    (else
      (set `self.Clockwise` true))))

(fn `UserConstructionScript`
  (bind (_returnvalue_roll _returnvalue_pitch _returnvalue_yaw) (`KismetMathLibrary.BreakRotator` (`self.K2_GetActorRotation`)))
  (`parent.UserConstructionScript`)
  (if (or (!= _returnvalue_roll 0.0) (!= _returnvalue_pitch 0.0))
    (`self.K2_SetActorRotation` (`KismetMathLibrary.MakeRotator` 0.0 0.0 _returnvalue_yaw))))