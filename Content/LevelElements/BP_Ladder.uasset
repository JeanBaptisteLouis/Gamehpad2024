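; BP_Ladder is a climbable ladder volume for BP_FirstPersonCharacter, driven by a Box overlap.
; Entering the box zeroes gravity, calls a zero-velocity launch and opens a Tick gate; leaving restores a fixed gravity scale and closes it.
; While open, Tick overwrites player 0's velocity from IA_Move input rotated to actor rotation, with the Y axis also driving vertical climb.
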(event `self.ReceiveTick`
  (params (DeltaSeconds :type "Float (single-precision)"))
  (bind _returnvalue (`GameplayStatics.GetPlayerCharacter` 0))
  (bind _returnvalue_2 (`|GetInputActionValue`))
  (bind (_x _y) (`KismetMathLibrary.BreakVector2D` (* _returnvalue_2 100.0)))
  (`/Engine/EditorBlueprintResources/StandardMacros.Gate` true :!label _label
    (:`Exit`
      (set `MovementComponent.Velocity` (`KismetMathLibrary.GreaterGreater_VectorRotator` (`KismetMathLibrary.MakeVector` _x _y (* (`.Y` (`KismetMathLibrary.BreakVector2D` _returnvalue_2)) 500.0)) (`self.K2_GetActorRotation` _returnvalue)) (`Character.CharacterMovement` _returnvalue)))))

(event `self.Box.OnComponentBeginOverlap`
  (params (OverlappedComponent :type "PrimitiveComponent Object Reference") (OtherActor :type "Actor Object Reference") (OtherComp :type "PrimitiveComponent Object Reference") (OtherBodyIndex :type Integer) (bFromSweep :type Boolean) (SweepResult :type "HitResult Structure (by ref)"))
  (bind _asbp_first_person_character (cast `/Game/FirstPerson/Blueprints/BP_FirstPersonCharacter` OtherActor))
  (set `CharacterMovementComponent.GravityScale` 0.0 (`Character.CharacterMovement` _asbp_first_person_character))
  (`Character.LaunchCharacter` _asbp_first_person_character (0.0 0.0 0.0) false false)
  (goto _label :!via `Open`))

(event `self.Box.OnComponentEndOverlap`
  (params (OverlappedComponent :type "PrimitiveComponent Object Reference") (OtherActor :type "Actor Object Reference") (OtherComp :type "PrimitiveComponent Object Reference") (OtherBodyIndex :type Integer))
  (bind _asbp_first_person_character (cast `/Game/FirstPerson/Blueprints/BP_FirstPersonCharacter` OtherActor))
  (set `CharacterMovementComponent.GravityScale` 2.0 (`Character.CharacterMovement` _asbp_first_person_character))
  (goto _label :!via `Close`))

(fn `UserConstructionScript`)