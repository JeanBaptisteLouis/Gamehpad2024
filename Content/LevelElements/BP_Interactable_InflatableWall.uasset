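; Interactable wall that inflates and deflates on alternating Interact events by scaling its Cube mesh.
; The construction script sizes a Box component from ExtendPoint, defining the inflated size.
; On inflate, it saves the Cube's world scale, then a timeline lerps relative scale from that toward the box extent divided by 50.
; The next interaction reverses the timeline from its end to restore the saved scale.
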(event `self._Interact`
  (`/Engine/EditorBlueprintResources/StandardMacros.FlipFlop`
    (:`A`
      (set `self.MeshScaleSave` (`SceneComponent.K2_GetComponentScale` (`self.Cube`)))
      (bind (_direction _newtrack_0) (`Timeline|Timeline_0` :!via `PlayFromStart` :!label _label)
        (:`Update`
          (`SceneComponent.SetRelativeScale3D` (`self.Cube`) (`KismetMathLibrary.VLerp` (`self.MeshScaleSave`) (/ (`BoxComponent.BoxExtent` (`self.Box`)) 50.0) _newtrack_0)))))
    (:`B`
      (goto _label :!via `ReverseFromEnd`))))

(fn `UserConstructionScript`
  (`parent.UserConstructionScript`)
  (`BoxComponent.SetBoxExtent` (`self.Box`) (`self.ExtendPoint`) true))